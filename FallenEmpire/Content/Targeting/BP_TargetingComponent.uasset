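; Targeting component that gives its owning Character a toggleable lock-on with left and right target switching.
; A sphere trace gathers BP_TargetingInterface actors, then line-trace hits are scored by alignment with camera forward.
; Switching filters hits by normal against camera right, releasing the lock if none is valid.
; While locked, Tick interpolates control rotation toward the target and the character follows controller rotation instead of movement direction.
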(event Custom|LockOnToActorRight
  (bind _targetingactors (CallFunction|FindLockTarget))
  (bind _closesttarget (CallFunction|FindClosestTargetontheRight _targetingactors))
  (Utilities|IsValid (Variables|Default|GetLockedOnActor)
    (:Is%20Valid
      (Utilities|IsValid _closesttarget
        (:Is%20Valid
          (Variables|Default|SetLockedOnActor _closesttarget))
        (:Is%20Not%20Valid
          (CallFunction|StopLockon))))))

(event Custom|OrientMovement
  (bind _characterref (Variables|Default|GetCharacterRef))
  (bind _charactermovement (Variables|/Script/Engine.Character|GetCharacterMovement _characterref))
  (Variables|/Script/Engine.CharacterMovementComponent|SetbOrientRotationToMovement _charactermovement true)
  (Variables|/Script/Engine.CharacterMovementComponent|SetbUseControllerDesiredRotation _charactermovement false))

(event Custom|StopLockOn
  (Variables|Default|SetLockedOnActor 0)
  (Variables|Default|SetLockedOn? false)
  (CallFunction|OrientMovement))

(event Custom|OrientCamera
  (bind _characterref (Variables|Default|GetCharacterRef))
  (bind _charactermovement (Variables|/Script/Engine.Character|GetCharacterMovement _characterref))
  (Variables|/Script/Engine.CharacterMovementComponent|SetbOrientRotationToMovement _charactermovement false)
  (Variables|/Script/Engine.CharacterMovementComponent|SetbUseControllerDesiredRotation _charactermovement true))

(event Custom|ToggleLockOn
  (if (Variables|Default|GetLockedOn?)
    (CallFunction|StopLockon)
    (else
      (CallFunction|LockontoTarget))))

(event Custom|LockOnToTarget
  (bind _targetingactors (CallFunction|FindLockTarget))
  (bind _closesttarget (CallFunction|FindClosestTarget _targetingactors))
  (Utilities|IsValid _closesttarget
    (:Is%20Valid
      (Variables|Default|SetLockedOnActor _closesttarget)
      (CallFunction|OrientCamera)
      (Variables|Default|SetLockedOn? true))))

(event Custom|LockOnToActorLeft
  (bind _targetingactors (CallFunction|FindLockTarget))
  (bind _closesttarget (CallFunction|FindClosestTargetontheLeft _targetingactors))
  (Utilities|IsValid (Variables|Default|GetLockedOnActor)
    (:Is%20Valid
      (Utilities|IsValid _closesttarget
        (:Is%20Valid
          (Variables|Default|SetLockedOnActor _closesttarget))
        (:Is%20Not%20Valid
          (CallFunction|StopLockon))))))

(event EventBeginPlay
  (bind _ascharacter (Utilities|Casting|CastToCharacter (Components|GetOwner)))
  (Variables|Default|SetCharacterRef _ascharacter)
  (Variables|Default|SetCameraRef (Actor|GetComponentbyClass (Variables|Default|GetCharacterRef) "/Script/Engine.CameraComponent")))

(event EventTick
  (params (DeltaSeconds :type Float%20%28single-precision%29))
  (if (Variables|Default|GetLockedOn?)
    (CallFunction|FaceLockedonActor)))

(fn FindLockTarget
  (bind _characterref (Variables|Default|GetCharacterRef))
  (bind _returnvalue (Transformation|GetActorLocation _characterref))
  (bind (_outhits _returnvalue_2) (Collision|MultiSphereTraceForObjects _returnvalue _returnvalue (Variables|Default|GetRadius) (Utilities|Array|MakeArray "ObjectTypeQuery7") false (Utilities|Array|MakeArray (Components|GetOwner)) "None"))
  (for _array_element _outhits
    (if (and _returnvalue_2 (Utilities|DoesObjectImplementInterface (.HitActor (Collision|BreakHitResult _array_element)) "/Game/Targeting/BP_TargetingInterface.BP_TargetingInterface_C"))
      (Utilities|Array|Add (LocalVariables|GetPotentialTargetingActors) (.HitActor (Collision|BreakHitResult _array_element)))))
  (return (LocalVariables|GetPotentialTargetingActors)))

(fn FindClosestTarget
  (params (Actors :type Array%20of%20Actor%20Object%20References))
  (for _array_element Actors
    (bind _returnvalue (Collision|LineTraceByChannel (Transformation|GetWorldLocation (Variables|Default|GetCameraRef)) (Transformation|GetActorLocation _array_element) "TraceTypeQuery1" false 0 "ForDuration"))
    (if _returnvalue
      (Math|Float|CompareFloat (CallFunction|CheckHowCloseTargetIstoPlayer _array_element) (LocalVariables|GetcompareTarget)
        (:>
          (LocalVariables|SetcompareTarget (CallFunction|CheckHowCloseTargetIstoPlayer _array_element))
          (LocalVariables|SetclosestLockTarget _array_element)))))
  (return (LocalVariables|GetclosestLockTarget)))

(fn CheckHowCloseTargetIstoPlayer
  (params (Target :type Actor%20Object%20Reference))
  (return (Math|Vector|DotProduct (Math|Vector|GetForwardVector (Variables|Default|GetCameraRef)) (Math|Rotator|GetRotationXVector (Math|Rotator|FindLookatRotation (Transformation|GetActorLocation (Variables|Default|GetCharacterRef)) (Transformation|GetActorLocation Target))))))

(fn FaceLockedonActor
  (bind _returnvalue (Utilities|Time|GetWorldDeltaSeconds))
  (bind _characterref (Variables|Default|GetCharacterRef))
  (bind _characterref_2 (Variables|Default|GetCharacterRef))
  (bind _lockedonactor (Variables|Default|GetLockedOnActor))
  (bind _interp_speed (Variables|Default|GetInterp%20Speed))
  (bind _returnvalue_2 (Pawn|GetController _characterref))
  (bind _returnvalue_3 (Transformation|GetActorLocation _lockedonactor))
  (bind _returnvalue_4 (Transformation|GetActorLocation _characterref_2))
  (bind _returnvalue_5 (Pawn|GetControlRotation _returnvalue_2 :!class /Script/Engine.Controller))
  (bind _returnvalue_6 (- _returnvalue_3 "0.000000,0.000000,120.000000"))
  (bind _returnvalue_7 (Math|Rotator|FindLookatRotation _returnvalue_4 _returnvalue_6))
  (bind _returnvalue_8 (Class|KismetMathLibrary|RInterptoConstant _returnvalue_5 _returnvalue_7 _returnvalue _interp_speed))
  (bind (_roll _pitch _yaw) (Math|Rotator|BreakRotator _returnvalue_8))
  (Pawn|SetControlRotation _returnvalue_2 (Math|Rotator|MakeRotator (.Roll (Math|Rotator|BreakRotator _returnvalue_5)) _pitch _yaw)))

(fn FindClosestTargetontheLeft
  (params (Actors :type Array%20of%20Actor%20Object%20References))
  (for _array_element Actors
    (bind (_outhit _returnvalue) (Collision|LineTraceByChannel (Transformation|GetWorldLocation (Variables|Default|GetCameraRef)) (Transformation|GetActorLocation _array_element) "TraceTypeQuery1" false 0 "ForDuration"))
    (if (Math|Boolean|ANDBoolean _returnvalue (> (Math|Vector|DotProduct (Math|Vector|GetRightVector (Variables|Default|GetCameraRef)) (.Normal (Collision|BreakHitResult _outhit))) 0.0) (!= (Variables|Default|GetLockedOnActor) _array_element))
      (Math|Float|CompareFloat (CallFunction|CheckHowCloseTargetIstoPlayer _array_element) (LocalVariables|GetcompareTarget)
        (:>
          (LocalVariables|SetcompareTarget (LocalVariables|GetcompareTarget))
          (LocalVariables|SetclosestLockTarget _array_element)))))
  (return (LocalVariables|GetclosestLockTarget)))

(fn FindClosestTargetontheRight
  (params (Actors :type Array%20of%20Actor%20Object%20References))
  (for _array_element Actors
    (bind (_outhit _returnvalue) (Collision|LineTraceByChannel (Transformation|GetWorldLocation (Variables|Default|GetCameraRef)) (Transformation|GetActorLocation _array_element) "TraceTypeQuery1" false 0 "ForDuration"))
    (if (Math|Boolean|ANDBoolean _returnvalue (< (Math|Vector|DotProduct (Math|Vector|GetRightVector (Variables|Default|GetCameraRef)) (.Normal (Collision|BreakHitResult _outhit))) 0.0) (!= (Variables|Default|GetLockedOnActor) _array_element))
      (Math|Float|CompareFloat (CallFunction|CheckHowCloseTargetIstoPlayer _array_element) (LocalVariables|GetcompareTarget)
        (:>
          (LocalVariables|SetcompareTarget (LocalVariables|GetcompareTarget))
          (LocalVariables|SetclosestLockTarget _array_element)))))
  (return (LocalVariables|GetclosestLockTarget)))